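; Character Blueprint for MonsterShooter that carries a sword and has debug-triggered visual test actions.
; On BeginPlay it spawns BP_Sword and snaps it to the right-hand socket on the mesh.
; Two debug keys each call a server-named RPC event, which forwards to a second RPC event: one swaps a mesh material to M_Lamp, the other plays the rifle shoot montage.
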(event Custom|RPC_ChangeMaterial
  (Rendering|Material|SetMaterial (Variables|Character|GetMesh) 1 "/Game/StarterContent/Props/Materials/M_Lamp.M_Lamp"))

(event Custom|RPC_Server_ChangeMaterial
  (CallFunction|RPCChangeMaterial))

(event Custom|RPC_RifeShootAnim
  (Animation|PlayAnimMontage "/Game/FirstPersonArms/Animations/FP_Rifle_Shoot_Montage.FP_Rifle_Shoot_Montage" 1.0 "None"))

(event Custom|RPC_Server_RifleShootAnim
  (CallFunction|RPCRifeShootAnim))

(event Collision|EventActorBeginOverlap
  (params (OtherActor :type Actor%20Object%20Reference)))

(event EventTick
  (params (DeltaSeconds :type Float%20%28single-precision%29)))

(event EventBeginPlay
  (bind _returnvalue (Game|SpawnActorfromClass "/Game/Blueprints/BP_Sword.BP_Sword_C" (Transformation|GetSocketTransform (Variables|Character|GetMesh) "hand_r_Sword_socket" "RTS_World") "Undefined" "MultiplyWithRoot" 0 0))
  (Transformation|AttachComponentToComponent _returnvalue (Variables|Character|GetMesh) "hand_r_Sword_socket" "SnapToTarget" "SnapToTarget" "SnapToTarget" true))

(event Input|KeyboardEvents|DebugKey2
  (params (Key :type Key%20Structure :default "None") (ActionValue :type Input%20Action%20Value%20Structure))
  (:Pressed
    (CallFunction|RPCServerChangeMaterial)))

(event Input|KeyboardEvents|DebugKey3
  (params (Key :type Key%20Structure :default "None") (ActionValue :type Input%20Action%20Value%20Structure))
  (:Pressed
    (CallFunction|RPCServerRifleShootAnim)))

(fn ConstructionScript)